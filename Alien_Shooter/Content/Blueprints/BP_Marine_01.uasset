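; BP_Marine_01 is a player-controlled marine with movement and weapon-fire effects.
; The forward and strafe axes add movement input along fixed world X and Y, independent of facing.
; Pressing fire activates the muzzle flash and spawns a stored 2D assault rifle sound, and releasing stops both, with no projectile or damage logic.
; The player rotation function is an empty stub that never runs.
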(event EventBeginPlay)

(event Input|ActionEvents|InputActionWeaponfire
  (params (Key :type Key%20Structure :default "None"))
  (:Pressed
    (Components|Activation|Activate (Variables|Default|Getmuzle%20flash) false)
    (bind _returnvalue (Audio|SpawnSound2D "/Game/Sounds/Weapon_AssaultRifle/Stereo/AssultRifleCompilation.AssultRifleCompilation" 1.0 1.0 0.0 0))
    (Variables|Default|Setsound%20shoot _returnvalue))
  (:Released
    (Components|Activation|Deactivate (Variables|Default|Getmuzle%20flash))
    (Audio|Components|Audio|Stop (Variables|Default|Getsound%20shoot))))

(event Input|AxisEvents|InputAxisMoveForward-Backward
  (params (AxisValue :type Float%20%28single-precision%29))
  (Pawn|Input|AddMovementInput "1.000000, 0, 0" AxisValue false))

(event Input|AxisEvents|InputAxisStrafeLeft-Right
  (params (AxisValue :type Float%20%28single-precision%29))
  (Pawn|Input|AddMovementInput "0,1.000000, 0" AxisValue false))

(fn ConstructionScript)

(fn UpdatePlayerRotation)